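; BP_Shuttle is a flyable shuttle pawn that the player possesses through a trigger interaction, attaching the character to the driver position.
; Toggling engines drives four BP_Engine child actors, sound, and timers for ground tracing and velocity-based engine tilt.
; Maneuvering requires engines on and enough altitude; Tick handles turning, banking, RPM audio and engine-off descent.
; Timelines and flip-flops animate landing gear and doors; another key toggles lights.
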(event OnComponentBeginOverlap(ControlTrigger)
  (params (OverlappedComponent :type Primitive%20Component%20Object%20Reference) (OtherActor :type Actor%20Object%20Reference) (OtherComp :type Primitive%20Component%20Object%20Reference) (OtherBodyIndex :type Integer) (bFromSweep :type Boolean) (SweepResult :type Hit%20Result%20Structure%20%28by%20ref%29))
  ;[1 0.1898 0.2996] Register player to the ship
  (if (not (Pawn|IsPlayerControlled self))
    (bind _player (Class|BPICharacter|IsPlayer(Message) OtherActor))
    (if _player
      (Class|BPICharacter|SetInteractable(Message) OtherActor self)
      (Utilities|IsValid (Variables|Default|GetInstructionWidget)
        (:Is%20Valid
          _)
        (:Is%20Not%20Valid
          (bind _returnvalue (UserInterface|CreateWidget "/Game/SpaceShip/Blueprints/WDG_Instructions.WDG_Instructions_C"))
          (Variables|Default|SetInstructionWidget _returnvalue)))
      (UserInterface|Viewport|AddtoViewport (Variables|Default|GetInstructionWidget) 0)
      (Default|SetInstructionText (Variables|Default|GetInstructionWidget) "Press 'F' to interact"))))

(event OnComponentEndOverlap(ControlTrigger)
  (params (OverlappedComponent :type Primitive%20Component%20Object%20Reference) (OtherActor :type Actor%20Object%20Reference) (OtherComp :type Primitive%20Component%20Object%20Reference) (OtherBodyIndex :type Integer))
  (bind _instructionwidget (Variables|Default|GetInstructionWidget))
  ;[1 0.1898 0.2996] Register player to the ship
  (if (not (Pawn|IsPlayerControlled self))
    (bind _player (Class|BPICharacter|IsPlayer(Message) OtherActor))
    (if _player
      (Class|BPICharacter|SetInteractable(Message) OtherActor)
      (Utilities|IsValid _instructionwidget
        (:Is%20Valid
          (if (UserInterface|Viewport|IsinViewport _instructionwidget)
            (Widget|RemovefromParent _instructionwidget)))))))

(event OnComponentBeginOverlap(Door1)
  (params (OverlappedComponent :type Primitive%20Component%20Object%20Reference) (OtherActor :type Actor%20Object%20Reference) (OtherComp :type Primitive%20Component%20Object%20Reference) (OtherBodyIndex :type Integer) (bFromSweep :type Boolean) (SweepResult :type Hit%20Result%20Structure%20%28by%20ref%29))
  ;[0.6552 0.2705 1] Toggle inner door
  (bind _player (Class|BPICharacter|IsPlayer(Message) OtherActor))
  (if _player
    (bind _newtrack_0 (Timeline|Timeline_3 Play)
      (:Update
        (Transformation|SetRelativeLocation (Variables|Default|GetDoorL) (Math|Vector|MakeVector 0.0 (Math|Float|Lerp 0.0 -105.0 _newtrack_0) 0.0) false true)
        (Transformation|SetRelativeLocation (Variables|Default|GetDoorR) (Math|Vector|MakeVector 0.0 (Math|Float|Lerp 0.0 105.0 _newtrack_0) 0.0) false false)))))

(event OnComponentEndOverlap(Door1)
  (params (OverlappedComponent :type Primitive%20Component%20Object%20Reference) (OtherActor :type Actor%20Object%20Reference) (OtherComp :type Primitive%20Component%20Object%20Reference) (OtherBodyIndex :type Integer))
  ;[0.6552 0.2705 1] Toggle inner door
  (bind _player (Class|BPICharacter|IsPlayer(Message) OtherActor))
  (if _player
    (bind _newtrack_0 (Timeline|Timeline_3 Reverse)
      (:Update
        (Transformation|SetRelativeLocation (Variables|Default|GetDoorL) (Math|Vector|MakeVector 0.0 (Math|Float|Lerp 0.0 -105.0 _newtrack_0) 0.0) false true)
        (Transformation|SetRelativeLocation (Variables|Default|GetDoorR) (Math|Vector|MakeVector 0.0 (Math|Float|Lerp 0.0 105.0 _newtrack_0) 0.0) false false)))))

(event OnComponentBeginOverlap(Door2)
  (params (OverlappedComponent :type Primitive%20Component%20Object%20Reference) (OtherActor :type Actor%20Object%20Reference) (OtherComp :type Primitive%20Component%20Object%20Reference) (OtherBodyIndex :type Integer) (bFromSweep :type Boolean) (SweepResult :type Hit%20Result%20Structure%20%28by%20ref%29))
  ;[1 0.4107 0.4906] Toggle inner door 2
  (bind _player (Class|BPICharacter|IsPlayer(Message) OtherActor))
  (if _player
    (bind _newtrack_0 (Timeline|Timeline_5 Play)
      (:Update
        (Transformation|SetRelativeLocation (Variables|Default|GetDoorL2) (Math|Vector|MakeVector 0.0 (Math|Float|Lerp 0.0 -105.0 _newtrack_0) 0.0) false true)
        (Transformation|SetRelativeLocation (Variables|Default|GetDoorR2) (Math|Vector|MakeVector 0.0 (Math|Float|Lerp 0.0 105.0 _newtrack_0) 0.0) false false)))))

(event OnComponentEndOverlap(Door2)
  (params (OverlappedComponent :type Primitive%20Component%20Object%20Reference) (OtherActor :type Actor%20Object%20Reference) (OtherComp :type Primitive%20Component%20Object%20Reference) (OtherBodyIndex :type Integer))
  ;[1 0.4107 0.4906] Toggle inner door 2
  (bind _player (Class|BPICharacter|IsPlayer(Message) OtherActor))
  (if _player
    (bind _newtrack_0 (Timeline|Timeline_5 Reverse)
      (:Update
        (Transformation|SetRelativeLocation (Variables|Default|GetDoorL2) (Math|Vector|MakeVector 0.0 (Math|Float|Lerp 0.0 -105.0 _newtrack_0) 0.0) false true)
        (Transformation|SetRelativeLocation (Variables|Default|GetDoorR2) (Math|Vector|MakeVector 0.0 (Math|Float|Lerp 0.0 105.0 _newtrack_0) 0.0) false false)))))

(event Custom|TurnShip
  (params (InputPin :type Float%20%28double-precision%29))
  ;[1 1 1] Turning
  (Utilities|CanManeuver
    (:true
      (bind _output_get (Variables|Default|SetYawTurning (Math|Float|Lerp (Variables|Default|GetYawTurning) (* InputPin (Utilities|Time|GetWorldDeltaSeconds) 2e+01) 0.05)))
      (if (not (Math|Float|NearlyEqual(Float) (Math|Float|Absolute(Float) _output_get) 0.0 0.01))
        (Transformation|AddLocalRotation (Variables|Default|GetCLM_Shuttle) (Math|Rotator|MakeRotator 0.0 0.0 _output_get) false false)))))

(event Custom|RandomizeSwayAngle
  (bind _returnvalue (Math|Random|RandomFloatinRange 0.0 0.04))
  (bind _returnvalue_2 (* _returnvalue -1.0))
  ;[0.3694 0.6763 1] add a sway effect
  (Utilities|FlowControl|FlipFlop
    (:A
      (Variables|Default|SetSwayingRate (Math|Rotator|MakeRotator _returnvalue _returnvalue 0.0)))
    (:B
      (Variables|Default|SetSwayingRate (Math|Rotator|MakeRotator _returnvalue_2 _returnvalue_2 0.0))))
  (Utilities|FlowControl|Delay (Math|Random|RandomFloatinRange 2.0 6.0)))

(event Custom|ToggleEngines
  (params (On/Off :type Boolean))
  ;[1 1 1] Turn On/Off Engins
  (if (!= On/Off (Variables|Default|GetEngineOn))
    (Utilities|FlowControl|DoOnce false :!label _label
      (:Completed
        (Utilities|ToggleEngineM (Variables|Default|GetBP_Engine_FL) On/Off)
        (Utilities|ToggleEngineM (Variables|Default|GetBP_Engine_BR) On/Off)
        (Utilities|ToggleEngineM (Variables|Default|GetBP_Engine_BL) On/Off)
        (Utilities|ToggleEngineM (Variables|Default|GetBP_Engine_FR) On/Off)
        (Utilities|FlowControl|Sequence
          (:then_0
            (Utilities|FlowControl|Delay 0.1)
            (Variables|Default|SetEngineOn On/Off)
            (Utilities|FlowControl|Sequence
              (:then_0
                (if (Variables|Default|GetEngineOn)
                  (Utilities|Time|SetTimerbyFunctionName 0 "TraceGround" 1.0 true)
                  (Utilities|Time|SetTimerbyFunctionName 0 "AdjustEngineRotation" 0.03 true)
                  (else
                    (Utilities|Time|ClearTimerbyFunctionName 0 "TraceGround")
                    (Utilities|Time|ClearTimerbyFunctionName 0 "AdjustEngineRotation"))))
              (:then_1
                (goto _label Reset))))
          (:then_1
            (|UpdateEngineSound On/Off)))))))

(event EventBeginPlay
  ;[1 0.5628 0.4828] Event Begin Play
  (CallFunction|RandomizeSwayAngle)
  ;;[1 0.7778 0] Assign light material
  (bind _returnvalue (Rendering|Material|CreateDynamicMaterialInstance (Variables|Default|GetLight) 0 0 "None" :!class /Script/Engine.PrimitiveComponent))
  (Variables|Default|SetLight1Mat _returnvalue)
  ;;[1 0.7778 0] Assign light material
  (bind _returnvalue_2 (Rendering|Material|CreateDynamicMaterialInstance (Variables|Default|GetLight1) 0 0 "None" :!class /Script/Engine.PrimitiveComponent))
  (Variables|Default|SetLight2Mat _returnvalue_2))

(event EventTick
  (params (DeltaSeconds :type Float%20%28single-precision%29))
  (CallFunction|TurnShip (Input|AxisValues|GetTurning))
  (CallFunction|SwayShip2)
  (if (Pawn|IsPlayerControlled)
    _
    (else
      (Pawn|Input|AddMovementInput (Variables|Default|GetShipVelocity) 1.0 false)))
  (bind _output_get (Variables|Default|SetSoundRPM (Math|Float|Lerp (Variables|Default|GetSoundRPM) (/ (Math|Vector|VectorLength (Transformation|GetVelocity)) (Variables|/Script/Engine.FloatingPawnMovement|GetMaxSpeed (Variables|Default|GetFloatingPawnMovement))) 0.01)))
  (Audio|Parameter|SetFloatParameter (Variables|Default|GetEngine) "RPM" _output_get :!class /Script/AudioExtensions.AudioParameterControllerInterface)
  (if (not (CallFunction|CheckGround))
    (if (not (Variables|Default|GetEngineOn))
      (Pawn|Input|AddMovementInput "0, 0,-1.000000" 1.0 false))))

(event EventUnpossessed
  (params (OldController :type Controller%20Object%20Reference))
  (bind _shipvelocity (Variables|Default|GetShipVelocity))
  (bind _floatingpawnmovement (Variables|Default|GetFloatingPawnMovement))
  ;[0.6782 1 0.436] on unpossessed
  (Pawn|SpawnDefaultController)
  (Variables|/Script/Engine.MovementComponent|SetVelocity _floatingpawnmovement _shipvelocity)
  (Class|MovementComponent|SetPlaneConstraintEnabled _floatingpawnmovement true)
  (Class|MovementComponent|SetPlaneConstraintfromVectors _floatingpawnmovement _shipvelocity (Transformation|GetActorUpVector)))

(event EventStartInteraction
  (params (InteractingActor :type Character%20Object%20Reference))
  (bind _instructionwidget (Variables|Default|GetInstructionWidget))
  ;[0.3033 0.3213 1] Player interact with the ship
  (Variables|Default|SetDriver InteractingActor)
  (Pawn|Possess (Game|GetPlayerController 0) self)
  (Collision|SetActorEnableCollision (Variables|Default|GetDriver) false)
  (Transformation|AttachComponentToComponent (Variables|Default|GetDriver) (Variables|Default|GetDriverPosition) "None" "SnapToTarget" "SnapToTarget" "KeepWorld" true)
  (Pawn|Components|CharacterMovement|DisableMovement (Variables|/Script/Engine.Character|GetCharacterMovement (Variables|Default|GetDriver)))
  (Class|MovementComponent|SetPlaneConstraintEnabled (Variables|Default|GetFloatingPawnMovement) false)
  (Utilities|IsValid _instructionwidget
    (:Is%20Valid
      (if (UserInterface|Viewport|IsinViewport _instructionwidget)
        (Widget|RemovefromParent _instructionwidget)))))

(event Input|AxisEvents|InputAxisFlying
  (params (AxisValue :type Float%20%28single-precision%29))
  ;[1 1 1] Flying Input
  (if (Variables|Default|GetEngineOn)
    (Pawn|Input|AddMovementInput "0, 0,1.000000" AxisValue false)))

(event Input|AxisEvents|InputAxisMoveForward/Backward
  (params (AxisValue :type Float%20%28single-precision%29))
  ;[0.05098 0.05098 0.05098] Horizontal Ship Movement
  (Utilities|CanManeuver
    (:true
      (Pawn|Input|AddMovementInput (Transformation|GetActorForwardVector) AxisValue false))))

(event Input|AxisEvents|InputAxisTurnRight/LeftGamepad
  (params (AxisValue :type Float%20%28single-precision%29))
  ;[0.05098 0.05098 0.05098] Camera Input - Gamepad
  (Pawn|Input|AddControllerYawInput (* AxisValue (Variables|Default|GetTurnRateGamepad) (Utilities|Time|GetWorldDeltaSeconds))))

(event Input|AxisEvents|InputAxisTurnRight/LeftMouse
  (params (AxisValue :type Float%20%28single-precision%29))
  ;[0.05098 0.05098 0.05098] Camera Input - Mouse
  (Pawn|Input|AddControllerYawInput AxisValue))

(event Input|AxisEvents|InputAxisLookUp/DownMouse
  (params (AxisValue :type Float%20%28single-precision%29))
  ;[0.05098 0.05098 0.05098] Camera Input - Mouse
  (Pawn|Input|AddControllerPitchInput AxisValue))

(event Input|AxisEvents|InputAxisLookUp/DownGamepad
  (params (AxisValue :type Float%20%28single-precision%29))
  ;[0.05098 0.05098 0.05098] Camera Input - Gamepad
  (Pawn|Input|AddControllerPitchInput (* AxisValue (Variables|Default|GetTurnRateGamepad) (Utilities|Time|GetWorldDeltaSeconds))))

(event Input|AxisEvents|InputAxisMoveRight/Left
  (params (AxisValue :type Float%20%28single-precision%29))
  ;[0.05098 0.05098 0.05098] Horizontal Ship Movement
  (Utilities|CanManeuver
    (:true
      (Pawn|Input|AddMovementInput (Transformation|GetActorRightVector) AxisValue false))))

(event Input|KeyboardEvents|L
  (params (Key :type Key%20Structure :default "None"))
  (bind _clm_shuttle (Variables|Default|GetCLM_Shuttle))
  (bind _clm_shuttle_2 (Variables|Default|GetCLM_Shuttle))
  (bind _returnvalue (Transformation|GetWorldRotation _clm_shuttle))
  (bind _returnvalue_2 (Transformation|GetWorldRotation _clm_shuttle_2))
  ;[1 1 1] Landing Gears
  (:Pressed
    (if (Variables|Default|GetEngineOn)
      (Utilities|FlowControl|FlipFlop
        (:A
          (bind _newtrack_0 (Timeline|Timeline_0 Play)
            (:Update
              (Transformation|SetRelativeRotation (Variables|Default|GetLandingGear_F) (Math|Rotator|MakeRotator 1.8e+02 (Math|Float|Lerp 5e+01 1.8e+02 _newtrack_0) 1.8e+02) false false)
              (Transformation|SetWorldRotation (Variables|Default|Getlanding_gierp_F) (Transformation|GetWorldRotation (Variables|Default|GetCLM_Shuttle)) false false)
              (Transformation|SetRelativeRotation (Variables|Default|GetLandingGear_L) (Math|Rotator|MakeRotator 1.8e+02 (Math|Float|Lerp 5e+01 1.8e+02 _newtrack_0) 9e+01) false false)
              (Transformation|SetRelativeRotation (Variables|Default|GetLandingGear_R) (Math|Rotator|MakeRotator 1.8e+02 (Math|Float|Lerp 5e+01 1.8e+02 _newtrack_0) 2.7e+02) false false)
              (Transformation|SetWorldRotation (Variables|Default|Getlanding_gierp_R) (Math|Rotator|MakeRotator (.roll _returnvalue_2) (.pitch _returnvalue_2) (+ (.yaw _returnvalue_2) 9e+01)) false false)
              (Transformation|SetWorldRotation (Variables|Default|Getlanding_gierp_L) (Math|Rotator|MakeRotator (.roll _returnvalue) (.pitch _returnvalue) (+ (.yaw _returnvalue) -9e+01)) false false))))
        (:B
          (Timeline|Timeline_0 Reverse))))))

(event Input|KeyboardEvents|O
  (params (Key :type Key%20Structure :default "None"))
  ;[0.2121 0.599 0.593] Door Open
  (:Pressed
    (Utilities|FlowControl|FlipFlop
      (:A
        (bind _newtrack_0 (Timeline|Timeline_1 Play)
          (:Update
            (Transformation|SetRelativeRotation (Variables|Default|GetDoorHinge) (Math|Rotator|MakeRotator 0.0 (Math|Float|Lerp 0.0 -9e+01 _newtrack_0) 0.0) false false))))
      (:B
        (Timeline|Timeline_1 Reverse)))))

(event Input|KeyboardEvents|K
  (params (Key :type Key%20Structure :default "None"))
  ;[1 0.3167 0] Toggle Lights
  (:Pressed
    (Utilities|FlowControl|FlipFlop
      (:A
        (Rendering|Material|SetScalarParameterValue (Variables|Default|GetLight2Mat) "Emissive" 5e+01 :!class /Script/Engine.MaterialInstanceDynamic)
        (Rendering|SetVisibility (Variables|Default|GetSpotLight) true false))
      (:B
        (Rendering|Material|SetScalarParameterValue (Variables|Default|GetLight2Mat) "Emissive" 0.0 :!class /Script/Engine.MaterialInstanceDynamic)
        (Rendering|SetVisibility (Variables|Default|GetSpotLight) false false)))))

(event Input|KeyboardEvents|T
  (params (Key :type Key%20Structure :default "None"))
  ;[1 1 1] Turn On/Off Engins
  (:Pressed
    (CallFunction|ToggleEngines (not (Variables|Default|GetEngineOn)))))

(fn ConstructionScript)

(fn SwayShip
  (bind _returnvalue (Transformation|GetActorRotation))
  (bind _returnvalue_2 (Utilities|Time|GetWorldDeltaSeconds))
  (bind _returnvalue_3 (Utilities|Time|GetWorldDeltaSeconds))
  (bind _swayingrate (Variables|Default|GetSwayingRate))
  (bind _returnvalue_4 (* _returnvalue_3 1e+01))
  (bind _returnvalue_5 (* _swayingrate _returnvalue_4))
  (bind (_roll _pitch) (Math|Rotator|BreakRotator _returnvalue_5))
  (if (> (Variables|Default|GetShipElevation) 1.5e+02)
    (Transformation|AddActorLocalRotation (Math|Rotator|MakeRotator (Math|Float|SelectFloat 0.0 _roll (> (Math|Float|Absolute(Float) (+ (.roll (Variables|Default|GetTotalOffset)) _roll)) 5.0)) (Math|Float|SelectFloat 0.0 _pitch (> (Math|Float|Absolute(Float) (+ (.pitch (Variables|Default|GetTotalOffset)) _pitch)) 2.0)) 0.0) false false)
    (Variables|Default|SetTotalOffset (Math|Rotator|MakeRotator (+ (Math|Float|SelectFloat 0.0 _roll (> (Math|Float|Absolute(Float) (+ (.roll (Variables|Default|GetTotalOffset)) _roll)) 5.0)) (.roll (Variables|Default|GetTotalOffset))) (+ (Math|Float|SelectFloat 0.0 _pitch (> (Math|Float|Absolute(Float) (+ (.pitch (Variables|Default|GetTotalOffset)) _pitch)) 2.0)) (.pitch (Variables|Default|GetTotalOffset))) 0.0))
    (else
      (Transformation|SetActorRotation (Math|Rotator|MakeRotator (Math|Interpolation|FInterpTo (.roll _returnvalue) 0.0 _returnvalue_2 1e+01) (Math|Interpolation|FInterpTo (.pitch _returnvalue) 0.0 _returnvalue_2 1e+01) (.yaw _returnvalue)))
      (Variables|Default|SetTotalOffset (Math|Rotator|MakeRotator (.roll _returnvalue) (.pitch _returnvalue) 0.0)))))

(fn TraceGround
  (bind _returnvalue (Transformation|GetActorLocation))
  (bind (_outhit _returnvalue_2) (Collision|LineTraceByChannel _returnvalue (+ _returnvalue "0.000000,0.000000,-1000.000000") "TraceTypeQuery1" false 0 "None"))
  (bind _output_get (Variables|Default|SetInFlyingElevation (not _returnvalue_2)))
  (if (not _output_get)
    (Variables|Default|SetShipElevation (.Distance (Collision|BreakHitResult _outhit)))))

(fn AdjustEngineRotation
  (Transformation|SetRelativeRotation (Variables|Default|GetBP_Engine_BL) (Math|Rotator|MakeRotator 0.0 (Math|Float|Clamp(Float) (+ (* (/ (Math|Vector|DotProduct (Transformation|GetVelocity) (Transformation|GetActorForwardVector)) (Variables|/Script/Engine.FloatingPawnMovement|GetMaxSpeed (Variables|Default|GetFloatingPawnMovement))) -9e+01) 9e+01) 0.0 135.0) 0.0) false false))

(fn SwayShip2
  (Transformation|SetActorRelativeRotation (Math|Rotator|MakeRotator (* (/ (Math|Vector|DotProduct (Transformation|GetVelocity) (Transformation|GetActorRightVector)) (Variables|/Script/Engine.FloatingPawnMovement|GetMaxSpeed (Variables|Default|GetFloatingPawnMovement))) 15.0) 0.0 (.yaw (Transformation|GetActorRotation)))))

(fn CheckGround
  (bind _returnvalue (Transformation|GetActorLocation))
  (bind _returnvalue_2 (Collision|LineTraceByChannel _returnvalue (+ _returnvalue "0.000000,0.000000,-100.000000") "TraceTypeQuery1" false 0 "None"))
  (return _returnvalue_2))