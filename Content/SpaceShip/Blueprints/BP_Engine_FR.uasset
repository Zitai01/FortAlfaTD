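; BP_Engine_FR is a spaceship engine Blueprint that adds a Niagara effect to the on/off behavior of its parent class.
; ToggleEngine runs the parent implementation first, then activates the Niagara1 component with a reset when switched on, or deactivates it when switched off.
; The construction script only calls the parent, and BeginPlay, overlap and Tick are disabled stubs.
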(event EventBeginPlay
  (|CallParentFunction) ; This node is disabled and will not be called.\nDrag off pins to build functionality.
)

(event Collision|EventActorBeginOverlap
  (params (OtherActor :type Actor%20Object%20Reference))
  (|CallParentFunction OtherActor) ; This node is disabled and will not be called.\nDrag off pins to build functionality.
)

(event EventTick
  (params (DeltaSeconds :type Float%20%28single-precision%29))
  (|CallParentFunction DeltaSeconds) ; This node is disabled and will not be called.\nDrag off pins to build functionality.
)

(event EventToggleEngine
  (params (On/Off :type Boolean))
  (bind _niagara1 (Variables|Default|GetNiagara1))
  (|CallParentFunction On/Off)
  (if On/Off
    (Components|Activation|Activate _niagara1 true)
    (else
      (Components|Activation|Deactivate _niagara1))))

(fn ConstructionScript
  (|CallParentFunction))