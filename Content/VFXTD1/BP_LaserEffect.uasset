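; Laser effect actor that fires a yellow Niagara beam along its forward vector and shows an impact effect where it hits.
; Each Tick runs a Camera-channel line trace, setting the beam's LaserEnd to the hit or trace end.
; The impact system moves to the hit location and is visible only on a blocking hit.
; Trace distance grows over time up to a large cap, so the beam extends progressively.
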(event EventBeginPlay)

(event Collision|EventActorBeginOverlap
  (params (OtherActor :type Actor%20Object%20Reference)))

(event EventTick
  (params (DeltaSeconds :type Float%20%28single-precision%29))
  (bind _returnvalue (Transformation|GetActorLocation))
  (Utilities|FlowControl|Sequence
    (:then_0
      (Effects|Components|ParticleSystem|SetColorParameter (Variables|Default|GetNiagaraLaserImpact) "Color" (Class|KismetMathLibrary|LinearColorYellow))
      (Variables|Default|SetTrace (+ _returnvalue (* (Transformation|GetActorForwardVector) (Variables|Default|GetDistance))))
      (bind _outhit (Collision|LineTraceByChannel _returnvalue (+ _returnvalue (* (Transformation|GetActorForwardVector) (Variables|Default|GetDistance))) "TraceTypeQuery2" false 0 "None"))
      (Variables|Default|SetbHit (.bblockinghit _outhit))
      (bind _output_get (Variables|Default|SetHitLocation (.location _outhit)))
      (Effects|Components|ParticleSystem|SetVectorParameter (Variables|Default|GetNiagaraLaser) "LaserEnd" (select (Variables|Default|GetbHit) (Variables|Default|GetHitLocation) (Variables|Default|GetTrace)))
      (Transformation|SetWorldLocation (Variables|Default|GetNiagaraLaserImpact) _output_get false false)
      (Rendering|SetVisibility (Variables|Default|GetNiagaraLaserImpact) (Variables|Default|GetbHit) false)
      (if (Variables|Default|GetbHit)
        (Variables|Default|SetDistance (Math|Vector|VectorLength (- (Variables|Default|GetTrace) (Transformation|GetActorLocation))))))
    (:then_1
      (if (< (Variables|Default|GetDistance) 5e+06)
        (Variables|Default|SetDistance (+ (Variables|Default|GetDistance) (* DeltaSeconds 1e+04)))))))

(fn ConstructionScript)